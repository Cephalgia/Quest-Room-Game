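; Note_BP is a note actor that opens an InfoPaper_BP widget when Q is pressed while overlapped.
; Begin overlap enables its input for player 0 and end overlap disables it, with no check on which actor overlaps.
; Q shows the widget in UI-only input mode, then copies the note's Image value into ImageIndex on DefaultPawn_BP, after the widget is already in the viewport.
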(event Collision|EventActorBeginOverlap
  (params (OtherActor :type Actor%20Object%20Reference))
  (Input|EnableInput (Game|GetPlayerController 0)))

(event Collision|EventActorEndOverlap
  (params (OtherActor :type Actor%20Object%20Reference))
  (Input|DisableInput 0))

(event Input|KeyboardEvents|Q
  (params (Key :type Key%20Structure :default "AnyKey"))
  (:Pressed
    (bind _returnvalue (UserInterface|CreateWidget "/Game/InfoPaper_BP.InfoPaper_BP_C"))
    (Input|SetInputModeUIOnly (Game|GetPlayerController 0) _returnvalue "DoNotLock")
    (UserInterface|Viewport|AddtoViewport _returnvalue 0)
    (bind _asdefault_pawn_bp (Utilities|Casting|CastToDefaultPawn_BP (Game|Player|GetPlayerPawn 0)))
    (Variables|/Game/DefaultPawn_BP.DefaultPawn_BP_C|SetImageIndex _asdefault_pawn_bp (Variables|Default|GetImage))))

(fn ConstructionScript)