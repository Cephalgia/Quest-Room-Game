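; CaesarMachine_BP is an interactable actor that opens a Caesar machine UI when the player uses it.
; Overlap enables the actor's input and shows a hint widget; ending overlap disables input and removes the hint.
; Pressing Q snaps the player pawn to a fixed offset from the machine and matches control rotation to the actor's.
; It then swaps the hint for the CaesarMachine_BP widget in UI-only input mode.
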(event Collision|EventActorBeginOverlap
  (params (OtherActor :type Actor%20Object%20Reference))
  (Input|EnableInput (Game|GetPlayerController 0))
  (bind _returnvalue (UserInterface|CreateWidget "/Game/Widgets/Hint_BP.Hint_BP_C"))
  (UserInterface|Viewport|AddtoViewport _returnvalue 0))

(event Collision|EventActorEndOverlap
  (params (OtherActor :type Actor%20Object%20Reference))
  (Input|DisableInput (Game|GetPlayerController 0))
  (Widget|RemovefromParent (stale Collision|EventActorBeginOverlap _returnvalue)))

(event Input|KeyboardEvents|Q
  (params (Key :type Key%20Structure :default "AnyKey"))
  (bind _returnvalue (Game|Player|GetPlayerPawn 0))
  (:Pressed
    (Transformation|SetActorLocation _returnvalue (+ (Transformation|GetActorLocation) (Math|Vector|MakeVector -5e+01 0.0 4e+01)) false false)
    (Pawn|SetControlRotation (Pawn|GetController _returnvalue) (Transformation|GetActorRotation))
    (Widget|RemovefromParent (stale Collision|EventActorBeginOverlap _returnvalue))
    (bind _returnvalue_2 (UserInterface|CreateWidget "/Game/Widgets/CaesarMachine_BP.CaesarMachine_BP_C"))
    (UserInterface|Viewport|AddtoViewport _returnvalue_2 0)
    (Input|SetInputModeUIOnly (Game|GetPlayerController 0) _returnvalue_2 "DoNotLock")))

(fn ConstructionScript)