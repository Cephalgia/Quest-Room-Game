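; An openable door actor that the player swings open by pressing E while overlapping it.
; Overlap events enable and disable input for the first player controller.
; The key press plays a DoorSwing timeline that adds its angle as yaw to the rotation saved at BeginPlay.
; An event track in the same timeline plays a door sound at the actor's location.
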(event EventBeginPlay
  (bind _output_get (Variables|Default|SetInitialRotation (Transformation|GetActorRotation))))

(event Collision|EventActorBeginOverlap
  (params (OtherActor :type Actor%20Object%20Reference))
  (Input|EnableInput (Game|GetPlayerController 0)))

(event Collision|EventActorEndOverlap
  (params (OtherActor :type Actor%20Object%20Reference))
  (Input|DisableInput (Game|GetPlayerController 0)))

(event Input|KeyboardEvents|E
  (params (Key :type Key%20Structure :default "AnyKey"))
  (:Pressed
    (bind _openangle (Timeline|DoorSwing Play)
      (:Update
        (Transformation|SetActorRotation (Math|Rotator|CombineRotators (Math|Rotator|MakeRotator 0.0 0.0 _openangle) (stale EventBeginPlay _output_get))))
      (:SoundTiming
        (Audio|PlaySoundatLocation "/Game/Audio/locked-door.locked-door" (Transformation|GetActorLocation))))))

(fn ConstructionScript)